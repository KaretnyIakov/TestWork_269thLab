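; Inventory component that tracks item counts and used slot totals for its owner, broadcasting item and weapon interactions.
; Adding routes weapons to a slot-specific event, while other items accumulate in a map keyed by item info.
; Slot usage is recalculated from each item's max stack size as counts change.
; Removal first applies the item's effect, such as messaging a heal to the owner, then returns the amount removed.
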(event EventBeginPlay)

(event EventTick
  (params (DeltaSeconds :type Float%20%28single-precision%29)))

(fn AddItemtoInventory
  (params (Item :type BP%20Item%20Object%20Reference))
  (bind _count (Default|GetCount Item))
  (bind _iteminfo (Variables|/Game/Inventory/BP_Item.BP_Item_C|GetItemInfo Item))
  (bind _inventory (Variables|Default|GetInventory))
  (bind _inventory_2 (Variables|Default|GetInventory))
  (bind _inventory_3 (Variables|Default|GetInventory))
  (bind (_value _returnvalue) (Utilities|Map|Find _inventory _iteminfo))
  (bind (_value_2 _returnvalue_2) (Utilities|Map|Find _inventory_3 _iteminfo))
  (if (Utilities|Enum|Equal(Enum) (Variables|/Game/Inventory/PDA_Item.PDA_Item_C|GetType (Variables|/Game/Inventory/BP_Item.BP_Item_C|GetItemInfo Item)) "NewEnumerator2")
    (CallFunction|AddWeapontoSlot Item)
    (else
      (if _returnvalue_2
        (LocalVariables|SetCurrentItemSlots (Math|Float|Ceil (/ (Math|Conversions|ToFloat(Integer) _value_2) (Math|Conversions|ToFloat(Integer) (Variables|/Game/Inventory/PDA_Item.PDA_Item_C|GetMaxCountInSlot _iteminfo))))))
      (if _returnvalue
        (Utilities|Map|Add _inventory_2 _iteminfo (+ _value _count))
        (Default|CallOnInteractwithItem _iteminfo (.Value (Utilities|Map|Find (Variables|Default|GetInventory) _iteminfo)))
        (else
          (Utilities|Map|Add _inventory_2 _iteminfo _count)
          (Default|CallOnInteractwithItem _iteminfo _count)))
      (LocalVariables|SetNewItemSlots (Math|Float|Ceil (/ (Math|Conversions|ToFloat(Integer) (.Value (Utilities|Map|Find (Variables|Default|GetInventory) _iteminfo))) (Math|Conversions|ToFloat(Integer) (Variables|/Game/Inventory/PDA_Item.PDA_Item_C|GetMaxCountInSlot _iteminfo)))))
      (Variables|Default|SetSlotsCount (+ (- (LocalVariables|GetNewItemSlots) (LocalVariables|GetCurrentItemSlots)) (Variables|Default|GetSlotsCount))))))

(fn RemoveItemfromInventory
  (params (Item :type PDA%20Item%20Object%20Reference) (Count :type Integer))
  (bind _inventory (Variables|Default|GetInventory))
  (bind (_value _returnvalue) (Utilities|Map|Find _inventory Item))
  (bind _returnvalue_2 (- _value Count))
  (CallFunction|ApplyItemEffect Item Count)
  (if _returnvalue
    (LocalVariables|SetCurrentItemSlots (Math|Float|Ceil (/ (Math|Conversions|ToFloat(Integer) (.Value (Utilities|Map|Find (Variables|Default|GetInventory) Item))) (Math|Conversions|ToFloat(Integer) (Variables|/Game/Inventory/PDA_Item.PDA_Item_C|GetMaxCountInSlot Item)))))
    (if (>= _returnvalue_2 0)
      (LocalVariables|SetCounter _returnvalue_2)
      (Utilities|Map|Add (Variables|Default|GetInventory) Item _returnvalue_2)
      (Default|CallOnInteractwithItem Item (LocalVariables|GetCounter))
      (LocalVariables|SetNewItemSlots (Math|Float|Ceil (/ (Math|Conversions|ToFloat(Integer) (.Value (Utilities|Map|Find (Variables|Default|GetInventory) Item))) (Math|Conversions|ToFloat(Integer) (Variables|/Game/Inventory/PDA_Item.PDA_Item_C|GetMaxCountInSlot Item)))))
      (Variables|Default|SetSlotsCount (- (Variables|Default|GetSlotsCount) (- (LocalVariables|GetCurrentItemSlots) (LocalVariables|GetNewItemSlots))))
      (return Count)
      (else
        (LocalVariables|SetCounter _value)
        (Utilities|Map|Remove (Variables|Default|GetInventory) Item)
        (Default|CallOnInteractwithItem Item)
        (Variables|Default|SetSlotsCount (- (Variables|Default|GetSlotsCount) (LocalVariables|GetCurrentItemSlots)))
        (return (LocalVariables|GetCounter))))
    (else
      (return 0))))

(fn ApplyItemEffect
  (params (Item :type PDA%20Item%20Object%20Reference) (Count :type Integer))
  (bind _itemtype (Default|Use Item))
  (switch Utilities|FlowControl|Switch|SwitchonEN_ItemTypes _itemtype
    (:NewEnumerator1
      (bind _aspda_item_heal (Utilities|Casting|CastToPDA_Item_Heal Item))
      (Class|HealthInterface|OnHeal(Message) (Components|GetOwner) (* (Variables|/Game/Inventory/Heals/PDA_Item_Heal.PDA_Item_Heal_C|GetHealCount _aspda_item_heal) Count)))))

(fn AddWeapontoSlot
  (params (Weapon :type BP%20Item%20Object%20Reference))
  (bind _asbp_weapon (Utilities|Casting|CastToBP_Weapon Weapon))
  (Default|CallOnInteractwithWeapon (Variables|/Game/Inventory/Weapon/Guns/PDA_Weapon.PDA_Weapon_C|GetWeaponSlot (Variables|/Game/Inventory/Weapon/Guns/BP_Weapon.BP_Weapon_C|GetWeaponInfo _asbp_weapon)) _asbp_weapon))