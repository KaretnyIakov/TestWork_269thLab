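; BP_Item is an inventory item actor that shows a mesh and exposes its count through GetCount.
; On BeginPlay it async-loads the soft mesh reference in ItemInfo and assigns it to ItemMesh.
; UseItem, run when the item is taken, flags it as used and hides the mesh without destroying the actor.
; The construction script records the actor's location as StartLocation.
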(event Custom|UseItem
  ;[0.03125 0.03125 0.03125] When Take Item
  (Variables|Default|SetIsUsed true)
  (Rendering|SetVisibility (Variables|Default|GetItemMesh) false false))

(event EventBeginPlay
  (bind _object (Utilities|AsyncLoadAsset (Variables|/Game/Inventory/PDA_Item.PDA_Item_C|GetMesh (Variables|Default|GetItemInfo)))
    (:Completed
      (bind _asstatic_mesh (Utilities|Casting|CastToStaticMesh _object))
      (Components|StaticMesh|SetStaticMesh (Variables|Default|GetItemMesh) _asstatic_mesh))))

(fn ConstructionScript
  (Variables|Default|SetStartLocation (Transformation|GetActorLocation)))

(fn GetCount
  (return (Variables|Default|GetCount)))