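; BP_Bullet is a gun projectile actor that deals damage on overlap and then destroys itself.
; When its mesh begins overlapping, it ignores its owner and any actor tagged as a bullet.
; Other actors with a HealthComponent and the HealthInterface receive the damage stored in BulletInfo through an interface message.
; The bullet is destroyed on any such overlap, whether or not damage was dealt.
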(event OnComponentBeginOverlap(BulletMesh)
  (params (OverlappedComponent :type Primitive%20Component%20Object%20Reference) (OtherActor :type Actor%20Object%20Reference) (OtherComp :type Primitive%20Component%20Object%20Reference) (OtherBodyIndex :type Integer) (bFromSweep :type Boolean) (SweepResult :type Hit%20Result%20Structure%20%28by%20ref%29))
  (if (not (Actor|ActorHasTag OtherActor "Bullet"))
    (if (!= (Components|GetOwner) OtherActor)
      (Utilities|IsValid (Actor|GetComponentbyClass OtherActor "/Script/TestTopDown.HealthComponent")
        (:Is%20Valid
          (if (Utilities|DoesObjectImplementInterface OtherActor "/Script/TestTopDown.HealthInterface")
            (Class|HealthInterface|OnDmd(Message) OtherActor (Variables|/Game/Inventory/Bullets/PDA_Item_Bullet.PDA_Item_Bullet_C|GetDmg (Variables|Default|GetBulletInfo)))))
        (:Is%20Not%20Valid
          _))
      (Actor|DestroyActor))))

(fn ConstructionScript)