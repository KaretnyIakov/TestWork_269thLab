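; BP_Weapon is a gun inventory item configured by a PDA_Weapon data asset that sets its muzzle point, firing mode, slot and bullet type.
; DoOnce gates limit burst mode to timed repeat shots and single mode to one shot until StopShooting.
; Shots spend clip ammo, play slot-based sound and spawn BP_Bullet after a short delay so the pawn can turn.
; Reloading requests ammo through a dispatcher, then a timer blocks firing.
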(event Custom|SpawnBullet
  ;[0.03125 0.03125 0.03125] Shooting / Bullet Spawn
  (Utilities|FlowControl|Delay 0.2) ; For pawn has time to turn to the target
  (CallFunction|SpawnBulletfromClasswithInfo))

(event Custom|ReloadWeaponTimer
  ;[0.03125 0.03125 0.03125] Reload Timer
  (Utilities|Time|SetTimerbyEvent (delegate Custom|ReloadCooldown) 2.0)
  (Variables|Default|SetReloading true))

(event Custom|ReloadCooldown
  ;[0.03125 0.03125 0.03125] Reload Timer
  (Variables|Default|SetReloading false))

(event EventBeginPlay
  (|CallParentFunction)
  ;[0.03125 0.03125 0.03125] Set the required Info
  (bind _aspda_weapon (Utilities|Casting|CastToPDA_Weapon (Variables|Default|GetItemInfo)))
  (Variables|Default|SetWeaponInfo _aspda_weapon)
  ;[0.03125 0.03125 0.03125] Set muzzle corresponding to the weapon
  (CallFunction|SetBulletStartPoint))

(event EventUseItem
  ;[0.03125 0.03125 0.03125] When Equip Weapon
  (Variables|Default|SetIsUsed true))

(event EventStopShooting
  ;[0.03125 0.03125 0.03125] Shooting / Bullet Spawn
  (Utilities|FlowControl|DoOnce false) ; enters at Reset
)

(event EventShooting
  ;[0.03125 0.03125 0.03125] Shooting / Bullet Spawn
  (if (not (Variables|Default|GetReloading))
    (if (> (Variables|Default|GetBulletsInClip) 0)
      (switch Utilities|FlowControl|Switch|SwitchonEN_ShootingModes (Variables|/Game/Inventory/Weapon/Guns/PDA_Weapon.PDA_Weapon_C|GetShootingMode (Variables|Default|GetWeaponInfo))
        (:NewEnumerator0
          (Utilities|FlowControl|DoOnce false :!label _label
            (:Completed
              (Utilities|FlowControl|Sequence
                (:then_0
                  (Utilities|FlowControl|Delay 0.2) ; Time interval between shots
                  (goto _label Reset))
                (:then_1
                  (Math|Integer|DecrementInt (Variables|Default|GetBulletsInClip)
                    (:%20%20
                      (CallFunction|SpawnBullet)
                      (CallFunction|PlayFireSound))))))))
        (:NewEnumerator1
          (Utilities|FlowControl|DoOnce false
            (:Completed
              (Math|Integer|DecrementInt (Variables|Default|GetBulletsInClip)
                (:%20%20
                  (CallFunction|SpawnBullet)
                  (CallFunction|PlayFireSound)))))))
      (else
        (Development|PrintString "No Bullets In Clip")))))

(fn ConstructionScript)

(fn TryReloadWeapon
  (bind _bulletcounttoreload (Default|ReloadWeapon (Variables|Default|GetWeaponInfo) (Variables|Default|GetBulletsInClip)))
  (Default|CallOnTryReloadWeapon self _bulletcounttoreload))

(fn ReloadWeapon
  (params (BulletCountToReload :type Integer))
  (Variables|Default|SetBulletsInClip (+ (Variables|Default|GetBulletsInClip) BulletCountToReload))
  (if (> BulletCountToReload 0)
    (CallFunction|ReloadWeaponTimer)))

(fn GetCount
  (return (|CallParentFunction)))

(fn SetBulletStartPoint
  (Transformation|SetRelativeLocation (Variables|Default|GetBulletStartPoint) (Variables|/Game/Inventory/Weapon/Guns/PDA_Weapon.PDA_Weapon_C|GetBulletStartPointCoords (Variables|Default|GetWeaponInfo)) false false))

(fn SpawnBulletfromClasswithInfo
  (bind _returnvalue (Components|GetOwner))
  (Game|SpawnActorfromClass "/Game/Inventory/Weapon/Guns/BP_Bullet.BP_Bullet_C" (Math|Transform|MakeTransform (Transformation|GetWorldLocation (Variables|Default|GetBulletStartPoint)) (Transformation|GetActorRotation _returnvalue) "1.000000,1.000000,1.000000") "Undefined" "MultiplyWithRoot" _returnvalue (Variables|/Game/Inventory/Weapon/Guns/PDA_Weapon.PDA_Weapon_C|GetWeaponBullletType (Variables|Default|GetWeaponInfo)) 0))

(fn PlayFireSound
  (bind _itemmesh (Variables|Default|GetItemMesh))
  (switch Utilities|FlowControl|Switch|SwitchonEN_WeaponSlotTypes (Variables|/Game/Inventory/Weapon/Guns/PDA_Weapon.PDA_Weapon_C|GetWeaponSlot (Variables|Default|GetWeaponInfo))
    (:NewEnumerator0
      (Audio|SpawnSoundAttached "/Game/Sounds/C_PistolFire.C_PistolFire" _itemmesh "None" "0, 0, 0" "0, 0, 0" "SnapToTarget" false 1.0 1.0 0.0 0 0))
    (:NewEnumerator1
      (Audio|SpawnSoundAttached "/Game/Sounds/C_RiffleFire.C_RiffleFire" _itemmesh "None" "0, 0, 0" "0, 0, 0" "SnapToTarget" false 1.0 1.0 0.0 0 0))))