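; Enemy turret Blueprint that automatically shoots at the player and can optionally patrol between two points.
; A detection sphere flags the player in range, and a looping timer line-traces for visibility, turns the mesh toward the player and spawns a bullet after a short delay.
; The construction script applies the patrol points, duration and detection radius.
; A health component feeds the overhead widget; death stops shooting and movement and hides the widget.
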(event OnComponentBeginOverlap(PlayerDetector)
  (params (OverlappedComponent :type Primitive%20Component%20Object%20Reference) (OtherActor :type Actor%20Object%20Reference) (OtherComp :type Primitive%20Component%20Object%20Reference) (OtherBodyIndex :type Integer) (bFromSweep :type Boolean) (SweepResult :type Hit%20Result%20Structure%20%28by%20ref%29))
  (if (Actor|ActorHasTag OtherActor "Player")
    (Variables|Default|SetPlayerInRad true)))

(event OnComponentEndOverlap(PlayerDetector)
  (params (OverlappedComponent :type Primitive%20Component%20Object%20Reference) (OtherActor :type Actor%20Object%20Reference) (OtherComp :type Primitive%20Component%20Object%20Reference) (OtherBodyIndex :type Integer))
  (if (Actor|ActorHasTag OtherActor "Player")
    (Variables|Default|SetPlayerInRad false)))

(event EventAttack
  ;[0.03125 0.03125 0.03125] Shooting
  (Utilities|FlowControl|Delay 0.2)
  (Game|SpawnActorfromClass "/Game/Inventory/Weapon/Guns/BP_Bullet.BP_Bullet_C" (Math|Transform|MakeTransform (Transformation|GetWorldLocation (Variables|Default|GetBulletStartPoint)) (Transformation|GetWorldRotation (Variables|Default|GetMesh)) "1.000000,1.000000,1.000000") "Undefined" "MultiplyWithRoot" self (Variables|/Game/Inventory/Weapon/Guns/PDA_Weapon.PDA_Weapon_C|GetWeaponBullletType (Variables|Default|GetWeaponInfo)) 0))

(event EventShooting
  ;[0.03125 0.03125 0.03125] Shooting
  (if (Variables|Default|GetPlayerInRad)
    (bind _canshoot (CallFunction|CheckPlayerVisibility))
    (if _canshoot
      (Transformation|SetWorldRotation (Variables|Default|GetMesh) (Math|Rotator|FindLookatRotation (Transformation|GetActorLocation) (Transformation|GetActorLocation (Game|Player|GetPlayerPawn 0))) false false)
      (Class|Enemy|Attack))))

(event EventOnDeath
  ;[0.03125 0.03125 0.03125] Health (Death) Events
  (Class|ShootingInterface|StopShooting)
  (Components|Activation|Deactivate (Variables|Default|GetInterpToMovement))
  (Development|SetHiddeninGame (Variables|Default|GetWidget) true false))

(event EventBeginPlay
  (|CallParentFunction)
  ;[0.03125 0.03125 0.03125] Add Health
  (bind _aswd_health (Utilities|Casting|CastToWD_Health (UserInterface|GetWidget (Variables|Default|GetWidget))))
  (Default|SetHealthComp _aswd_health (Variables|Default|GetHealthComponent))
  ;[0.03125 0.03125 0.03125] Time Auto Shooting
  (bind _returnvalue (Utilities|Time|SetTimerbyEvent (delegate EventShooting) 1.0 true))
  (Variables|Default|SetTimer _returnvalue)
  ;[0.03125 0.03125 0.03125] Stop movement if not movable
  (if (not (Variables|Default|GetMovable))
    (Components|Activation|Deactivate (Variables|Default|GetInterpToMovement))))

(event EventStopShooting
  ;[0.03125 0.03125 0.03125] Shooting
  (Utilities|Time|PauseTimerbyHandle (Variables|Default|GetTimer)))

(fn ConstructionScript
  (bind _interptomovement (Variables|Default|GetInterpToMovement))
  (Variables|/Script/Engine.InterpToMovementComponent|SetControlPoints _interptomovement (Utilities|Array|MakeArray (Utilities|Struct|MakeInterpControlPoint (Variables|Default|GetPoint_01) true) (Utilities|Struct|MakeInterpControlPoint (Variables|Default|GetPoint_02) true)))
  (Variables|/Script/Engine.InterpToMovementComponent|SetDuration _interptomovement (Variables|Default|GetDuration))
  (Components|Sphere|SetSphereRadius (Variables|Default|GetPlayerDetector) (Variables|Default|GetPlayerDetectionRadius) true))

(fn CheckPlayerVisibility
  (bind _outhit (Collision|LineTraceByChannel (Transformation|GetWorldLocation (Variables|Default|GetMesh)) (Transformation|GetActorLocation (Pawn|GetControlledPawn (Game|GetPlayerController 0))) "TraceTypeQuery1" false (Utilities|Array|MakeArray self) "None"))
  (if (.bBlockingHit (Collision|BreakHitResult _outhit))
    (if (Actor|ActorHasTag (.HitActor (Collision|BreakHitResult _outhit)) "Player")
      (return true)
      (else
        (return false)))
    (else
      (return true))))